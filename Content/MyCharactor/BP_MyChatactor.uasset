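; Player character Blueprint that handles movement, look, jump and sprint through Enhanced Input.
; On BeginPlay it adds the IMC_MyCharacter mapping context to the owning player's input subsystem.
; Movement follows control rotation, with pitch zeroed for forward motion, while sprint switches max walk speed between running and walking values.
; A hard-wired T key, outside the input actions, plays a stand-to-cover montage on the mesh.
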(event `self.ReceiveBeginPlay`
  (bind _asplayer_controller (cast `PlayerController` (`self.GetController`)))
  (`EnhancedInputSubsystemInterface.AddMappingContext` (pcsubsystem `EnhancedInputLocalPlayerSubsystem` _asplayer_controller) "/Game/MyCharactor/MyInput/IMC_MyCharacter.IMC_MyCharacter" 0 (struct)))

(event `EnhancedInput|/Game/MyCharactor/MyInput/IA_MyCharacter_Jump`
  (params (ActionValue :type Boolean) (ElapsedSeconds :type "Float (double-precision)") (TriggeredSeconds :type "Float (double-precision)") (InputAction :type "InputAction Object Reference" :default "/Game/MyCharactor/MyInput/IA_MyCharacter_Jump.IA_MyCharacter_Jump"))
  (:`Started`
    (`self.Jump`))
  (:`Completed`
    (`self.StopJumping`)))

(event `EnhancedInput|/Game/MyCharactor/MyInput/IA_MyChartacter_Movement`
  (params (ActionValue :type "Vector2D Structure") (ElapsedSeconds :type "Float (double-precision)") (TriggeredSeconds :type "Float (double-precision)") (InputAction :type "InputAction Object Reference" :default "/Game/MyCharactor/MyInput/IA_MyChartacter_Movement.IA_MyChartacter_Movement"))
  (:`Triggered`
    (`self.AddMovementInput` (`KismetMathLibrary.GetForwardVector` (`KismetMathLibrary.MakeRotator` (.roll (`self.GetControlRotation`)) 0.0 (.yaw (`self.GetControlRotation`)))) ActionValue_Y)
    (`self.AddMovementInput` (`KismetMathLibrary.GetRightVector` (`self.GetControlRotation`)) ActionValue_X)))

(event `EnhancedInput|/Game/MyCharactor/MyInput/IA_MyChartacter_Movement_Look`
  (params (ActionValue :type "Vector2D Structure") (ElapsedSeconds :type "Float (double-precision)") (TriggeredSeconds :type "Float (double-precision)") (InputAction :type "InputAction Object Reference" :default "/Game/MyCharactor/MyInput/IA_MyChartacter_Movement_Look.IA_MyChartacter_Movement_Look"))
  (:`Triggered`
    (`self.AddControllerPitchInput` ActionValue_Y)
    (`self.AddControllerYawInput` ActionValue_X)))

(event `EnhancedInput|/Game/MyCharactor/MyInput/IA_MyChartacter_Sprint`
  (params (ActionValue :type Boolean) (ElapsedSeconds :type "Float (double-precision)") (TriggeredSeconds :type "Float (double-precision)") (InputAction :type "InputAction Object Reference" :default "/Game/MyCharactor/MyInput/IA_MyChartacter_Sprint.IA_MyChartacter_Sprint"))
  (:`Started`
    (set `CharacterMovementComponent.MaxWalkSpeed` 600.0 (`self.CharacterMovement`)))
  (:`Completed`
    (set `CharacterMovementComponent.MaxWalkSpeed` 150.0 (`self.CharacterMovement`))))

(event `Key|T`
  (params (Key :type "Key Structure"))
  (:`Pressed`
    (`|PlayMontage` (`self.Mesh`) "/Game/Characters/MyCharactor/Animation/stand_to_cover_Montage.stand_to_cover_Montage")))

(fn `UserConstructionScript`)